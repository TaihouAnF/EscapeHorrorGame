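; BP_ChainRust is a construction-time tool that lays chain link meshes along an editable spline.
; The construction script adds a static mesh every Spacing × ChainSize units, aligned to the spline's rotation and scaled by ChainSize.
; A Ceil-minus-Floor parity test rolls every other link 90 degrees so neighbours interlock.
; It also moves a Scene component to the last spline point; the event graph has no active logic.
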(event EventBeginPlay)

(event Collision|EventActorBeginOverlap
  (params (OtherActor :type Actor%20Object%20Reference)))

(event EventTick
  (params (DeltaSeconds :type Float%20%28single-precision%29)))

(fn ConstructionScript
  (bind _spacing (Variables|Components|GetSpacing))
  (bind _chainsize (Variables|Components|GetChainSize))
  (bind _spline (Variables|Default|GetSpline))
  (bind _returnvalue (* _spacing _chainsize))
  (Transformation|SetWorldLocation (Variables|Default|GetScene) (Spline|GetLocationatSplinePoint _spline (- (Spline|GetNumberOfSplinePoints _spline) 1) "World") false false)
  (for _index (range 0 (Math|Float|Floor (/ (Spline|GetSplineLength _spline) _returnvalue)))
    (AddComponent|AddStaticMeshComponent false (Math|Transform|MakeTransform (Spline|GetLocationatDistanceAlongSpline _spline (* _index _returnvalue) "Local") (Math|Rotator|MakeRotator (+ (.roll (Spline|GetRotationatDistanceAlongSpline _spline (* _index _returnvalue) "Local")) (Utilities|Select :Index (- (Math|Float|Ceil (* _index 0.5)) (Math|Float|Floor (* _index 0.5))) :Option%200 0.0 :Option%201 9e+01)) (.pitch (Spline|GetRotationatDistanceAlongSpline _spline (* _index _returnvalue) "Local")) (.yaw (Spline|GetRotationatDistanceAlongSpline _spline (* _index _returnvalue) "Local"))) (* (Variables|Components|GetRelative%20Transform%20Scale) (Variables|Components|GetChainSize))))))