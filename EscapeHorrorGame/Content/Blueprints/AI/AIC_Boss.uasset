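; AI controller for the boss that starts the BT_Boss behavior tree on possession.
; Events for hearing, losing and chasing the player write two Blackboard booleans through key-name variables, one for hear and one for chase.
; LostPlayer clears only the hear flag, while ShouldLosePlayer clears both chase and hear.
; The controller does no detection itself, so these events rely on outside callers.
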(event Custom|HeardPlayer
  ;[1 1 1] Set HearPlayer? True of False
  (AI|Components|Blackboard|SetValueasBool (Variables|Default|GetBlackboard) (Variables|Default|GetKeyName_hear) true))

(event Custom|LostPlayer
  ;[1 1 1] Set HearPlayer? True of False
  (AI|Components|Blackboard|SetValueasBool (Variables|Default|GetBlackboard) (Variables|Default|GetKeyName_hear) false))

(event Custom|ShouldChasePlayer
  ;[1 1 1] Set IfPlayerMoveNear True or False
  (AI|Components|Blackboard|SetValueasBool (Variables|Default|GetBlackboard) (Variables|Default|GetKeyName_Chase) true))

(event Custom|ShouldLosePlayer
  (bind _blackboard (Variables|Default|GetBlackboard))
  ;[1 1 1] Set IfPlayerMoveNear True or False
  (AI|Components|Blackboard|SetValueasBool _blackboard (Variables|Default|GetKeyName_Chase) false)
  (AI|Components|Blackboard|SetValueasBool _blackboard (Variables|Default|GetKeyName_hear) false))

(event EventPossess
  (params (PossessedPawn :type Pawn%20Object%20Reference))
  (AI|RunBehaviorTree "/Game/Blueprints/AI/BT_Boss.BT_Boss"))

(fn ConstructionScript)