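; Boss monster that plays a "don't move" sonar game with the player, reporting the results to AIC_Boss.
; Each listen event snapshots player position, shows warning UI, pulses echolocation on a looping timer, then compares positions after four seconds.
; The default pass signals heard or lost; the angrier post-approach pass decides chase or lose.
; It also forwards reset and inactivate, exposes its patrol route, and on kill spawns camera-facing UI before firing a dispatcher.
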(event Custom|MakeSound
  (bind _spawn_transform (Variables|Default|GetSpawn%20Transform))
  (bind _aicontrollerref (Variables|Default|GetAIControllerRef))
  ;[1 1 1] Generate Waves of Sonar and Movement detect within seconds, Works as the default behavior for the monster
  (Variables|Default|SetPlayerLastPos (Transformation|GetActorLocation (Variables|Default|GetPlayerRef)))
  (bind _returnvalue (Game|SpawnActorfromClass "/Game/Blueprints/UI/BP_SpawnUIElementDontMove.BP_SpawnUIElementDontMove_C" _spawn_transform "Undefined" "MultiplyWithRoot" 0 0))
  (Variables|Default|SetUI_DontMove _returnvalue)
  (Audio|PlaySoundatLocation "/Game/Sounds/Monster/CUE/EchoLocation.EchoLocation" (Transformation|GetActorLocation) "0, 0, 0" 1.0 1.0 0.0 "/Game/Sounds/Monster/MonsterAttenuation.MonsterAttenuation" 0 0 0)
  (bind _returnvalue_2 (Utilities|Time|SetTimerbyFunctionName 0 "SpawnEchoLocation" 0.8 true))
  (Utilities|FlowControl|Delay 4.0)
  (Utilities|Time|PauseTimerbyHandle _returnvalue_2)
  (bind _result (CallFunction|DetectPlayerMovementwithOutput))
  (Actor|DestroyActor (Variables|Default|GetUI_DontMove))
  (bind _returnvalue_3 (Game|SpawnActorfromClass "/Game/Blueprints/UI/BP_SpawnUIElementCanMove.BP_SpawnUIElementCanMove_C" _spawn_transform "Undefined" "MultiplyWithRoot" 0 0))
  (Variables|Default|SetUI_CanMove _returnvalue_3)
  (Utilities|FlowControl|Delay 2.0)
  (Actor|DestroyActor (Variables|Default|GetUI_CanMove))
  (if _result
    (Default|HeardPlayer _aicontrollerref)
    (else
      (Default|LostPlayer _aicontrollerref))))

(event Custom|MakeSoundAfterApproach
  (bind _aicontrollerref (Variables|Default|GetAIControllerRef))
  (bind _spawn_transform (Variables|Default|GetSpawn%20Transform))
  ;[1 1 1] Generate Waves of Sonar and Movement Detect after the Monster's first time finding the player
  (Variables|Default|SetPlayerLastPos (Transformation|GetActorLocation (Variables|Default|GetPlayerRef)))
  (bind _returnvalue (Game|SpawnActorfromClass "/Game/Blueprints/UI/BP_SpawnUIElementDontMoveAgain.BP_SpawnUIElementDontMoveAgain_C" _spawn_transform "Undefined" "MultiplyWithRoot" 0 0))
  (Variables|Default|SetUI_DontMoveAgain _returnvalue)
  (Audio|PlaySoundatLocation "/Game/Sounds/Monster/CUE/AngrySound.AngrySound" (Transformation|GetActorLocation) "0, 0, 0" 1.0 1.0 0.0 "/Game/Sounds/Monster/MonsterAttenuation.MonsterAttenuation" 0 0 0)
  (bind _returnvalue_2 (Utilities|Time|SetTimerbyFunctionName 0 "SpawnEchoLocation" 0.8 true))
  (Utilities|FlowControl|Delay 4.0)
  (Utilities|Time|PauseTimerbyHandle _returnvalue_2)
  (bind _result (CallFunction|DetectPlayerMovementwithOutput))
  (Actor|DestroyActor (Variables|Default|GetUI_DontMoveAgain))
  (bind _returnvalue_3 (Game|SpawnActorfromClass "/Game/Blueprints/UI/BP_SpawnUIElementCanMove.BP_SpawnUIElementCanMove_C" _spawn_transform "Undefined" "MultiplyWithRoot" 0 0))
  (Variables|Default|SetUI_CanMove _returnvalue_3)
  (Utilities|FlowControl|Delay 2.0)
  (Actor|DestroyActor (Variables|Default|GetUI_CanMove))
  (if _result
    (Default|ShouldChasePlayer _aicontrollerref)
    (else
      (Default|ShouldLosePlayer _aicontrollerref))))

(event Custom|ResetBackToLast
  (bind _aicontrollerref (Variables|Default|GetAIControllerRef))
  ;[1 1 1] Resetting the attributes
  (Default|ShouldLosePlayer _aicontrollerref)
  (Default|LostPlayer _aicontrollerref))

(event Custom|OnKill
  (bind _playerref (Variables|Default|GetPlayerRef))
  (bind _returnvalue (Actor|GetComponentbyClass _playerref "/Script/Engine.CameraComponent"))
  ;[1 1 1] Event dispatcher for Restart UI to show, First spawn the UI actor
  (bind _returnvalue_2 (Game|SpawnActorfromClass "/Game/Blueprints/UI/BP_SpawnUIElementAfterKill.BP_SpawnUIElementAfterKill_C" (Math|Conversions|ToTransform(Vector) (+ (Transformation|GetWorldLocation _returnvalue) (* (Math|Vector|GetForwardVector _returnvalue) (Variables|Default|GetUIDistance)))) "Undefined" "MultiplyWithRoot" 0 0))
  (Transformation|SetActorRotation _returnvalue_2 (Math|Rotator|FindLookatRotation (Transformation|GetActorLocation _returnvalue_2) (Transformation|GetWorldLocation _returnvalue)))
  (Default|CallOnTriggerKill))

(event Custom|Inactivate
  (Default|ShouldInactive (Variables|Default|GetAIControllerRef)))

(event EventBeginPlay
  (Variables|Default|SetPlayerRef (Game|Player|GetPlayerPawn 0))
  (bind _returnvalue (Actor|GetActorOfClass "/Game/Blueprints/AI/AIC_Boss.AIC_Boss_C"))
  (Variables|Default|SetAIControllerRef _returnvalue))

(fn ConstructionScript)

(fn SpawnEchoLocation
  (Default|SpawnEcho (Variables|Default|GetBPC_SpawnEchoLocation) 5e+03))

(fn DetectPlayerMovementwithOutput
  (return (Utilities|Operators|NotEqual(!=) (Variables|Default|GetPlayerLastPos) (Transformation|GetActorLocation (Variables|Default|GetPlayerRef)) 0.5)))

(fn GetPatrolRoute
  (return (Variables|Default|GetPatrolRoute)))