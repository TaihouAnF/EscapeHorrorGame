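; Restart component for the VR echolocation game that returns the player to the last checkpoint through its Restart event.
; It moves the pawn to the position stored in VRGameMode, then resets the VR pawn's height.
; It calls activation and lose-player functions on the boss AI controller, then clears the post-kill UI spawner.
; The first AIController found must be AIC_Boss, otherwise the UI cleanup is skipped for a VR pawn.
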(event Custom|Restart
  (bind _returnvalue (Game|Player|GetPlayerPawn 0))
  ;[1 1 1] Restart feature, remember to change game mode to VR game mode after testing
  (bind _asvrgame_mode (Utilities|Casting|CastToVRGameMode (Game|GetGameMode))
    (:then
      (Transformation|SetActorLocation _returnvalue (Variables|/Game/VRTemplate/Blueprints/VRGameMode.VRGameMode_C|GetLastCheckpointPos _asvrgame_mode) false false)
      (bind _asvrpawn_modified (Utilities|Casting|CastToVRPawn_Modified _returnvalue)
        (:then
          (Default|ResetHeight _asvrpawn_modified)
          (bind _returnvalue_2 (Actor|GetActorOfClass "/Script/AIModule.AIController"))
          (bind _asaic_boss (Utilities|Casting|CastToAIC_Boss _returnvalue_2))
          (Default|SHouldActive _asaic_boss)
          (Default|ShouldLosePlayer _asaic_boss)
          (Default|LostPlayer _asaic_boss))
        (:CastFailed
          _))
      (bind _returnvalue_3 (Actor|GetActorOfClass "/Game/Blueprints/UI/BP_SpawnUIElementAfterKill.BP_SpawnUIElementAfterKill_C"))
      (Default|DestroyAfterRestart _returnvalue_3))
    (:CastFailed
      (Development|PrintString "Failed to cast game mode"))))