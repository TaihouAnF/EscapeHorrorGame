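; Gesture-casting component that drives the owner's GestureTracker to trigger a Kamehameha beam attack from drawn gestures.
; BeginPlay adds the test input context, starts gesture drawing and loads saved gestures into an ID list.
; Holding IA_Recognition records a gesture; on release, gesture 0 spawns a charging beam at the tracker and gesture 1 fires it.
; Helper functions save gesture data, select the ID to record and swap the preview mesh.
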(event Input|EnhancedActionEvents|EnhancedInputActionIA_Recognition
  (params (ActionValue :type Boolean) (ElapsedSeconds :type Float%20%28double-precision%29) (TriggeredSeconds :type Float%20%28double-precision%29) (InputAction :type Input%20Action%20Object%20Reference :default "/Game/Blueprints/GestureRecognition/Inputs/IA_Recognition.IA_Recognition"))
  (bind _gesturetracker (Variables|Default|GetGestureTracker))
  (:Started
    (Class|GestureTracker|StartRecognition _gesturetracker 0 true false))
  (:Completed
    (bind _id (Class|GestureTracker|FinishRecognition _gesturetracker)
      (:Recognized
        (switch int _id
          (:0
            (bind _returnvalue (Game|SpawnActorfromClass "/Game/Blueprints/GestureRecognition/Kamehameha/BP_Kamehameha.BP_Kamehameha_C" (Transformation|GetWorldTransform (Variables|Default|GetGestureTracker)) "Undefined" "MultiplyWithRoot" 0 0))
            (Default|StartCharging _returnvalue)
            (Variables|Default|SetCurBeam _returnvalue))
          (:1
            (Default|Fire (Variables|Default|GetCurBeam))))))))

(event EventTick
  (params (DeltaSeconds :type Float%20%28single-precision%29)))

(event EventBeginPlay
  (Variables|Default|SetGestureTracker (Actor|GetComponentbyClass (Components|GetOwner) "/Script/GestureTrackerVR.GestureTracker"))
  (Input|AddMappingContext (PlayerController|LocalPlayerSubsystems|GetEnhancedInputLocalPlayerSubsystem (Game|GetPlayerController 0)) "/Game/Blueprints/GestureRecognition/Inputs/IMC_TestGesture.IMC_TestGesture" 0 "(bIgnoreAllPressedKeysUntilRelease=True,bForceImmediately=False,bNotifyUserSettings=False)")
  (Class|GestureTracker|StartDrawTrackedGesture (Variables|Default|GetGestureTracker))
  (Class|GestureTracker|StartDrawPredictedGesture (Variables|Default|GetGestureTracker) 0 0 0 0 true)
  (Class|GestureTracker|LoadGestures (Variables|Default|GetGestureTracker) "Data/Gestures/GestureData"
    (:Success
      (for _array_element (Class|GestureTracker|GetIds (Variables|Default|GetGestureTracker))
        (Utilities|Array|Add (Variables|Default|GetGestureIdArray) _array_element)))))

(fn SaveGestures
  (Class|GestureTracker|SaveGestures (Variables|Default|GetGestureTracker) "Data/Gestures/GestureData"
    (:Success
      (Development|PrintString "Save gestures success!"))
    (:Failed
      (Development|PrintString "Save gestures fail!"))))

(fn WriteGesturebyId
  (params (Id :type Integer) (GesturePreview :type Gesture%20Mesh%20Component%20Object%20Reference))
  (Utilities|FlowControl|Sequence
    (:then_0
      (if (== Id (Utilities|Array|Length (Variables|Default|GetGestureIdArray)))
        (Utilities|Array|Add (Variables|Default|GetGestureIdArray) Id)))
    (:then_1
      (if (not (< Id 0))
        (bind _output_get (Variables|Default|SetCurRecordId Id))
        (Development|PrintString (Utilities|String|Append "Set gesture: " (Utilities|String|ToString(Integer) _output_get)))))
    (:then_2
      (Utilities|IsValid (Variables|Default|GetGesturePreviewMesh)
        (:Is%20Valid
          (Components|DestroyComponent (Variables|Default|GetGesturePreviewMesh)))
        (:Is%20Not%20Valid
          _))
      (Variables|Default|SetGesturePreviewMesh GesturePreview))))