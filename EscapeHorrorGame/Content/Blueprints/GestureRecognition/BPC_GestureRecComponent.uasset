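; Component that records, saves and recognizes gestures on its owning VR pawn, where recognized gestures shrink or grow the pawn.
; On BeginPlay it loads saved gestures into the owner's GestureTracker and opens the WB_GestureEditor widget with their IDs.
; Enhanced Input actions drive recording into the current ID, set by number keys or WriteGestureById, and recognition.
; The Z key or SaveGestures writes gesture data back to file.
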(event Input|EnhancedActionEvents|EnhancedInputActionIA_Record
  (params (ActionValue :type Boolean) (ElapsedSeconds :type Float%20%28double-precision%29) (TriggeredSeconds :type Float%20%28double-precision%29) (InputAction :type Input%20Action%20Object%20Reference :default "/Game/Blueprints/GestureRecognition/Inputs/IA_Record.IA_Record"))
  (bind _enablerecord (Variables|Default|GetEnableRecord))
  (bind _gesturetracker (Variables|Default|GetGestureTracker))
  (:Triggered
    (if _enablerecord
      (Development|PrintString "recording")))
  (:Started
    (if _enablerecord
      (Class|GestureTracker|StartRecording _gesturetracker false)))
  (:Completed
    (if _enablerecord
      (Class|GestureTracker|FinishRecording _gesturetracker (Variables|Default|GetCurRecordId) (Variables|Default|GetCurRecordName)
        (:Recorded
          (Development|PrintString "Recorded"))))))

(event Input|EnhancedActionEvents|EnhancedInputActionIA_Recognition
  (params (ActionValue :type Boolean) (ElapsedSeconds :type Float%20%28double-precision%29) (TriggeredSeconds :type Float%20%28double-precision%29) (InputAction :type Input%20Action%20Object%20Reference :default "/Game/Blueprints/GestureRecognition/Inputs/IA_Recognition.IA_Recognition"))
  (bind _vrpawn (Variables|Default|GetVRPawn))
  (:Started
    (if (Variables|Default|GetEnableRecognition)
      (Class|GestureTracker|StartRecognition (Variables|Default|GetGestureTracker) 0 true false)))
  (:Completed
    (if (Variables|Default|GetEnableRecognition)
      (bind _id (Class|GestureTracker|FinishRecognition (Variables|Default|GetGestureTracker))
        (:Recognized
          (switch int _id
            (:0
              (Default|Shrink _vrpawn))
            (:1
              (Default|Grow _vrpawn))))))))

(event EventTick
  (params (DeltaSeconds :type Float%20%28single-precision%29)))

(event EventBeginPlay
  (Variables|Default|SetGestureTracker (Actor|GetComponentbyClass (Components|GetOwner) "/Script/GestureTrackerVR.GestureTracker"))
  (Class|GestureTracker|StartDrawTrackedGesture (Variables|Default|GetGestureTracker))
  (Class|GestureTracker|StartDrawPredictedGesture (Variables|Default|GetGestureTracker) 0 0 0 0 true)
  (Class|GestureTracker|LoadGestures (Variables|Default|GetGestureTracker) "Data/Gestures/GestureData"
    (:Success
      (for _array_element (Class|GestureTracker|GetIds (Variables|Default|GetGestureTracker))
        (Utilities|Array|Add (Variables|Default|GetGestureIdArray) _array_element))
      (Development|PrintString "Gesture Loaded Successfully")
      (bind _returnvalue (UserInterface|CreateWidget "/Game/Blueprints/GestureRecognition/WB_GestureEditor.WB_GestureEditor_C"))
      (UserInterface|Viewport|AddtoViewport _returnvalue 0)
      (Default|Initialize _returnvalue (Variables|Default|GetGestureIdArray) self)
      (Input|SetInputModeGameandUI (Game|GetPlayerController 0) _returnvalue "DoNotLock" true false)
      (bind _asvrpawn_modified (Utilities|Casting|CastToVRPawn_Modified (Components|GetOwner)))
      (Variables|Default|SetVRPawn _asvrpawn_modified))))

(event Input|KeyboardEvents|Z
  (params (Key :type Key%20Structure :default "None"))
  (:Pressed
    (Class|GestureTracker|SaveGestures (Variables|Default|GetGestureTracker) "Data/Gestures/GestureData"
      (:Success
        (Development|PrintString "Save gesture successfully"))
      (:Failed
        (Development|PrintString "Save gesture failed")))))

(event Input|KeyboardEvents|0
  (params (Key :type Key%20Structure :default "None"))
  (:Pressed
    (Variables|Default|SetCurRecordId 0)))

(event Input|KeyboardEvents|1
  (params (Key :type Key%20Structure :default "None"))
  (:Pressed
    (Variables|Default|SetCurRecordId 1)))

(event Input|KeyboardEvents|2
  (params (Key :type Key%20Structure :default "None"))
  (:Pressed
    (Variables|Default|SetCurRecordId 2)))

(event Input|KeyboardEvents|3
  (params (Key :type Key%20Structure :default "None"))
  (:Pressed
    (Variables|Default|SetCurRecordId 3)))

(fn SaveGestures
  (Class|GestureTracker|SaveGestures (Variables|Default|GetGestureTracker) "Data/Gestures/GestureData"
    (:Success
      (Development|PrintString "Save gestures success!"))
    (:Failed
      (Development|PrintString "Save gestures fail!"))))

(fn WriteGesturebyId
  (params (Id :type Integer) (GesturePreview :type Gesture%20Mesh%20Component%20Object%20Reference))
  (Utilities|FlowControl|Sequence
    (:then_0
      (if (== Id (Utilities|Array|Length (Variables|Default|GetGestureIdArray)))
        (Utilities|Array|Add (Variables|Default|GetGestureIdArray) Id)))
    (:then_1
      (if (not (< Id 0))
        (bind _output_get (Variables|Default|SetCurRecordId Id))
        (Development|PrintString (Utilities|String|Append "Set gesture: " (Utilities|String|ToString(Integer) _output_get)))))
    (:then_2
      (Utilities|IsValid (Variables|Default|GetGesturePreviewMesh)
        (:Is%20Valid
          (Components|DestroyComponent (Variables|Default|GetGesturePreviewMesh)))
        (:Is%20Not%20Valid
          _))
      (Variables|Default|SetGesturePreviewMesh GesturePreview))))