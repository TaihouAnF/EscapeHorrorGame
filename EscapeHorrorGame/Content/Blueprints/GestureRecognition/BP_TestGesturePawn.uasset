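; Test pawn for recording and recognizing mouse-drawn gestures that trigger abilities.
; Each tick moves its GestureTracker to the cursor hit point, while Enhanced Input starts and finishes recording or recognition.
; BeginPlay loads saved gestures and opens WB_GestureEditor; helper functions set the record ID, swap the preview mesh and save to file.
; Recognized IDs spawn or fire a Kamehameha beam, or shrink or grow matching actors.
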(event Input|EnhancedActionEvents|EnhancedInputActionIA_Record
  (params (ActionValue :type Boolean) (ElapsedSeconds :type Float%20%28double-precision%29) (TriggeredSeconds :type Float%20%28double-precision%29) (InputAction :type Input%20Action%20Object%20Reference :default "/Game/Blueprints/GestureRecognition/Inputs/IA_Record.IA_Record"))
  (bind _gesturetracker (Variables|Default|GetGestureTracker))
  (:Started
    (Class|GestureTracker|StartRecording _gesturetracker false))
  (:Completed
    (Class|GestureTracker|FinishRecording _gesturetracker (Variables|Default|GetCurRecordId) (Variables|Default|GetCurRecordName)
      (:Recorded
        (Development|PrintString "Recorded")))))

(event Input|EnhancedActionEvents|EnhancedInputActionIA_Recognition
  (params (ActionValue :type Boolean) (ElapsedSeconds :type Float%20%28double-precision%29) (TriggeredSeconds :type Float%20%28double-precision%29) (InputAction :type Input%20Action%20Object%20Reference :default "/Game/Blueprints/GestureRecognition/Inputs/IA_Recognition.IA_Recognition"))
  (bind _gesturetracker (Variables|Default|GetGestureTracker))
  (:Started
    (Class|GestureTracker|StartRecognition _gesturetracker 0 true false))
  (:Completed
    (bind _id (Class|GestureTracker|FinishRecognition _gesturetracker)
      (:Recognized
        (switch int _id
          (:0
            (bind _returnvalue (Game|SpawnActorfromClass "/Game/Blueprints/GestureRecognition/Kamehameha/BP_Kamehameha.BP_Kamehameha_C" (Transformation|GetWorldTransform (Variables|Default|GetGestureTracker)) "Undefined" "MultiplyWithRoot" 0 0))
            (Default|StartCharging _returnvalue)
            (Variables|Default|SetCurBeam _returnvalue))
          (:1
            (Default|Fire (Variables|Default|GetCurBeam)))
          (:2
            (bind _outactors (Actor|GetAllActorsOfClass "/Game/VRTemplate/Blueprints/OurStuff/Shrinker.Shrinker_C"))
            (for _array_element _outactors
              (Default|Shrink _array_element)))
          (:3
            (bind _outactors_2 (Actor|GetAllActorsOfClass "/Game/VRTemplate/Blueprints/OurStuff/Grower.Grower_C"))
            (for _array_element_2 _outactors_2
              (Default|Grow _array_element_2))))))))

(event EventBeginPlay
  (bind _gesturetracker (Variables|Default|GetGestureTracker))
  (bind _gesturetracker_2 (Variables|Default|GetGestureTracker))
  (Input|AddMappingContext (PlayerController|LocalPlayerSubsystems|GetEnhancedInputLocalPlayerSubsystem (Game|GetPlayerController 0)) "/Game/Blueprints/GestureRecognition/Inputs/IMC_TestGesture.IMC_TestGesture" 0 "(bIgnoreAllPressedKeysUntilRelease=True,bForceImmediately=False,bNotifyUserSettings=False)")
  (Class|GestureTracker|StartDrawTrackedGesture _gesturetracker)
  (Class|GestureTracker|StartDrawPredictedGesture _gesturetracker 0 0 0 0 true)
  (Class|GestureTracker|LoadGestures _gesturetracker_2 "Data/Gestures/GestureData"
    (:Success
      (for _array_element (Class|GestureTracker|GetIds _gesturetracker_2)
        (Utilities|Array|Add (Variables|Default|GetGestureIdArray) _array_element))
      (Development|PrintString "Gesture Loaded Successfully")
      (bind _returnvalue (UserInterface|CreateWidget "/Game/Blueprints/GestureRecognition/WB_GestureEditor.WB_GestureEditor_C"))
      (UserInterface|Viewport|AddtoViewport _returnvalue 0)
      (Default|Initialize _returnvalue (Variables|Default|GetGestureIdArray) self)
      (Input|SetInputModeGameandUI (Game|GetPlayerController 0) _returnvalue "DoNotLock" true false))))

(event Collision|EventActorBeginOverlap
  (params (OtherActor :type Actor%20Object%20Reference)))

(event EventTick
  (params (DeltaSeconds :type Float%20%28single-precision%29))
  (bind _returnvalue (Game|GetPlayerController 0))
  (bind _hitresult (Game|Player|GetHitResultUnderCursorbyChannel _returnvalue "TraceTypeQuery1" true))
  (bind _location (Collision|BreakHitResult _hitresult))
  (Transformation|SetWorldLocation (Variables|Default|GetGestureTracker) _location false false)
  (Rendering|Debug|DrawDebugSphere _location 1e+01 12 "(R=1.000000,G=0.000000,B=0.008842,A=1.000000)" 0.0 1.0))

(fn ConstructionScript)

(fn SaveGestures
  (Class|GestureTracker|SaveGestures (Variables|Default|GetGestureTracker) "Data/Gestures/GestureData"
    (:Success
      (Development|PrintString "Save gestures success!"))
    (:Failed
      (Development|PrintString "Save gestures fail!"))))

(fn WriteGesturebyId
  (params (Id :type Integer) (GesturePreview :type Gesture%20Mesh%20Component%20Object%20Reference))
  (Utilities|FlowControl|Sequence
    (:then_0
      (if (== Id (Utilities|Array|Length (Variables|Default|GetGestureIdArray)))
        (Utilities|Array|Add (Variables|Default|GetGestureIdArray) Id)))
    (:then_1
      (if (not (< Id 0))
        (bind _output_get (Variables|Default|SetCurRecordId Id))
        (Development|PrintString (Utilities|String|Append "Set gesture: " (Utilities|String|ToString(Integer) _output_get)))))
    (:then_2
      (Utilities|IsValid (Variables|Default|GetGesturePreviewMesh)
        (:Is%20Valid
          (Components|DestroyComponent (Variables|Default|GetGesturePreviewMesh)))
        (:Is%20Not%20Valid
          _))
      (Variables|Default|SetGesturePreviewMesh GesturePreview))))