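; Kamehameha energy beam actor that charges, fires and fades, with C starting the charge and F firing.
; Tick runs three flag-driven stages: BeamRoot grows to a maximum size, Cylinder stretches along Z to full length, then after a one-second timer BeamRoot shrinks away and both scales reset.
; Charge and fire sounds play at the beam root, alongside a toggled charging sound component.
; StopCharging and Reset are empty stubs.
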(event Custom|CustomEvent_0
  ;[1 1 1] Fire
  (Variables|Default|SetIsFading true))

(event EventBeginPlay
  (bind _returnvalue (Audio|SpawnSoundatLocation "/Game/Sounds/Kamehameha/kame_charging.kame_charging" (Transformation|GetWorldLocation (Variables|Default|GetBeamRoot)) "0, 0, 0" 1.0 1.0 0.0 0 0 false))
  (bind _output_get (Variables|Default|SetChargingSound _returnvalue))
  (Components|Activation|ToggleActive _output_get)
  (Input|EnableInput (Game|GetPlayerController 0)))

(event Collision|EventActorBeginOverlap
  (params (OtherActor :type Actor%20Object%20Reference)))

(event EventTick
  (params (DeltaSeconds :type Float%20%28single-precision%29))
  (bind _cylinder (Variables|Default|GetCylinder))
  (Utilities|FlowControl|Sequence
    (:then_0
      ;[1 1 1] Charging
      (if (Variables|Default|GetIsCharging)
        (if (< (.X (Math|Vector|BreakVector (Transformation|GetWorldScale (Variables|Default|GetBeamRoot)))) (Variables|Default|GetBeamMaxSize))
          (Transformation|SetWorldScale3D (Variables|Default|GetBeamRoot) (+ (* (Math|Vector|MakeVector DeltaSeconds DeltaSeconds DeltaSeconds) (Variables|Default|GetChargeSpeed)) (Transformation|GetWorldScale (Variables|Default|GetBeamRoot))))
          (else
            (Variables|Default|SetIsCharging false)))))
    (:then_1
      ;[1 1 1] Fire
      (if (Variables|Default|GetIsFiring)
        (if (< (.Z (Math|Vector|BreakVector (Variables|/Script/Engine.SceneComponent|GetRelativeScale3D (Variables|Default|GetCylinder)))) (Variables|Default|GetBeamMaxLength))
          (Transformation|SetRelativeScale3D _cylinder (Math|Vector|MakeVector 0.5 0.5 (+ (* DeltaSeconds (Variables|Default|GetBeamSpeed)) (.Z (Math|Vector|BreakVector (Variables|/Script/Engine.SceneComponent|GetRelativeScale3D _cylinder))))))
          (else
            (Variables|Default|SetIsFiring false)
            (Utilities|Time|SetTimerbyEvent (delegate Custom|CustomEvent_0) 1.0)))))
    (:then_2
      (CallFunction|Fade (Variables|Default|GetIsFading) DeltaSeconds))))

(event Input|KeyboardEvents|F
  (params (Key :type Key%20Structure))
  (:Pressed
    (CallFunction|Fire)))

(event Input|KeyboardEvents|C
  (params (Key :type Key%20Structure))
  (:Pressed
    (CallFunction|StartCharging)))

(fn ConstructionScript)

(fn StartCharging
  (Variables|Default|SetIsCharging true)
  (Audio|PlaySoundatLocation "/Game/Sounds/Kamehameha/kame_charge_1_.kame_charge_1_" (Transformation|GetWorldLocation (Variables|Default|GetBeamRoot)) "0, 0, 0" 1.0 1.0 0.0 0 0 0 0)
  (Components|Activation|SetActive (Variables|Default|GetChargingSound) true false))

(fn StopCharging)

(fn Fire
  (Variables|Default|SetIsFiring true)
  (Components|Activation|ToggleActive (Variables|Default|GetChargingSound))
  (Audio|PlaySoundatLocation "/Game/Sounds/Kamehameha/kame_fire.kame_fire" (Transformation|GetWorldLocation (Variables|Default|GetBeamRoot)) "0, 0, 0" 1.0 1.0 0.0 0 0 0 0))

(fn Fade
  (params (IsFading :type Boolean) (DeltaTime :type Float%20%28double-precision%29))
  (bind _beamroot (Variables|Default|GetBeamRoot))
  (if IsFading
    (Transformation|SetRelativeScale3D _beamroot (- (Variables|/Script/Engine.SceneComponent|GetRelativeScale3D _beamroot) (* (Math|Vector|MakeVector DeltaTime DeltaTime DeltaTime) (Variables|Default|GetFadeSpeed))))
    (if (<= (.X (Math|Vector|BreakVector (Variables|/Script/Engine.SceneComponent|GetRelativeScale3D (Variables|Default|GetBeamRoot)))) 0.0)
      (Variables|Default|SetIsFading false)
      (Transformation|SetRelativeScale3D (Variables|Default|GetBeamRoot) "0, 0, 0")
      (Transformation|SetRelativeScale3D (Variables|Default|GetCylinder) "0.500000,0.500000,0.000000"))))

(fn Reset)