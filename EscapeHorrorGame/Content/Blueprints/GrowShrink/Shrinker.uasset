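; Shrinker actor that shrinks nearby objects carrying a SizeIsFluid component to a tenth of their scale.
; Sphere overlap stores an unshrunk object's component as the target, while BeginPlay and any end overlap reset it to the SacraficialBlock's component as a placeholder.
; The Shrink event skips that placeholder, scales the overlapped component, sets IsShrunk to block repeat shrinking and activates SizeChangingSmoke.
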(event OnComponentBeginOverlap(Sphere)
  (params (OverlappedComponent :type Primitive%20Component%20Object%20Reference) (OtherActor :type Actor%20Object%20Reference) (OtherComp :type Primitive%20Component%20Object%20Reference) (OtherBodyIndex :type Integer) (bFromSweep :type Boolean) (SweepResult :type Hit%20Result%20Structure%20%28by%20ref%29))
  (bind _returnvalue (Actor|GetComponentbyClass OtherActor "/Game/Blueprints/GrowShrink/SizeIsFluid.SizeIsFluid_C"))
  (if (Utilities|IsValid _returnvalue)
    (if (not (Variables|/Game/Blueprints/GrowShrink/SizeIsFluid.SizeIsFluid_C|GetIsShrunk _returnvalue))
      (Variables|Default|SetOther _returnvalue))))

(event Custom|Shrink
  (if (!= (Variables|Default|GetOther) (Variables|/Game/Blueprints/GrowShrink/SacraficialBlock.SacraficialBlock_C|GetSizeIsFluid (stale Collision|EventActorEndOverlap _returnvalue)))
    (if (not (Variables|/Game/Blueprints/GrowShrink/SizeIsFluid.SizeIsFluid_C|GetIsShrunk (Actor|GetComponentbyClass (stale OnComponentBeginOverlap(Sphere) OtherActor) "/Game/Blueprints/GrowShrink/SizeIsFluid.SizeIsFluid_C")))
      (Transformation|SetWorldScale3D (stale OnComponentBeginOverlap(Sphere) OtherComp) (Math|Vector|MakeVector (* (.X (Math|Vector|BreakVector (Transformation|GetWorldScale (stale OnComponentBeginOverlap(Sphere) OtherComp)))) 0.1) (* (.Y (Math|Vector|BreakVector (Transformation|GetWorldScale (stale OnComponentBeginOverlap(Sphere) OtherComp)))) 0.1) (* (.Z (Math|Vector|BreakVector (Transformation|GetWorldScale (stale OnComponentBeginOverlap(Sphere) OtherComp)))) 0.1)))
      (Variables|/Game/Blueprints/GrowShrink/SizeIsFluid.SizeIsFluid_C|SetIsShrunk (Variables|Default|GetOther) true)
      (Components|Activation|Activate (Variables|Default|GetSizeChangingSmoke) true))))

(event Collision|EventActorEndOverlap
  (params (OtherActor :type Actor%20Object%20Reference))
  (bind _returnvalue (Actor|GetActorOfClass "/Game/Blueprints/GrowShrink/SacraficialBlock.SacraficialBlock_C"))
  (Variables|Default|SetOther (Variables|/Game/Blueprints/GrowShrink/SacraficialBlock.SacraficialBlock_C|GetSizeIsFluid _returnvalue)))

(event EventBeginPlay
  (bind _returnvalue (Actor|GetActorOfClass "/Game/Blueprints/GrowShrink/SacraficialBlock.SacraficialBlock_C"))
  (Variables|Default|SetOther (Variables|/Game/Blueprints/GrowShrink/SacraficialBlock.SacraficialBlock_C|GetSizeIsFluid _returnvalue)))

(fn ConstructionScript)