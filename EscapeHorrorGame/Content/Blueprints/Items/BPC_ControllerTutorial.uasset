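; Actor component that shows a controller grab tutorial while the player is near its owning item.
; On BeginPlay it caches the owner's hint widget component and sphere collision, then binds to the sphere's overlap events.
; When the player pawn enters the sphere it spawns a grab tutorial UI actor, and destroys that actor when the pawn leaves.
; The cached hint widget component is not used afterwards.
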(event Custom|BeginOverlap
  (params (OverlappedComponent :type Primitive%20Component%20Object%20Reference) (OtherActor :type Actor%20Object%20Reference) (OtherComp :type Primitive%20Component%20Object%20Reference) (OtherBodyIndex :type Integer) (bFromSweep :type Boolean) (SweepResult :type Hit%20Result%20Structure%20%28by%20ref%29))
  (if (== OtherActor (Game|Player|GetPlayerPawn 0))
    (bind _returnvalue (Game|SpawnActorfromClass "/Game/Blueprints/UI/BP_SpawnUIElementControllerTutorial_Grab.BP_SpawnUIElementControllerTutorial_Grab_C" (Math|Transform|MakeTransform "0, 0, 0" "0, 0, 0" "1.000000,1.000000,1.000000") "AlwaysSpawn" "MultiplyWithRoot" 0 0))
    (Variables|Default|SetGrabUI _returnvalue)))

(event Custom|EndOverlap
  (params (OverlappedComponent :type Primitive%20Component%20Object%20Reference) (OtherActor :type Actor%20Object%20Reference) (OtherComp :type Primitive%20Component%20Object%20Reference) (OtherBodyIndex :type Integer))
  (bind _grabui (Variables|Default|GetGrabUI))
  (if (== OtherActor (Game|Player|GetPlayerPawn 0))
    (Utilities|IsValid _grabui
      (:Is%20Valid
        (Actor|DestroyActor _grabui)))))

(event EventBeginPlay
  (bind _returnvalue (Components|GetOwner))
  (Utilities|FlowControl|Sequence
    (:then_0
      (Variables|Default|SetHintWidgetComponent (Actor|GetComponentbyClass _returnvalue "/Game/Blueprints/Items/BPC_HintWidgetComponent.BPC_HintWidgetComponent_C"))
      (Variables|Default|SetSphereCollision (Actor|GetComponentbyClass _returnvalue "/Script/Engine.SphereComponent")))
    (:then_1
      (Collision|BindEventtoOnComponentBeginOverlap (Variables|Default|GetSphereCollision) (delegate Custom|BeginOverlap))
      (Collision|BindEventtoOnComponentEndOverlap (Variables|Default|GetSphereCollision) (delegate Custom|EndOverlap)))))