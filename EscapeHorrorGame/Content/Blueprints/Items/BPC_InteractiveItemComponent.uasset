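; An actor component for interactive items that shows a hint widget when the player is near.
; On BeginPlay it finds the owner's hint widget, sphere collision and optional grab component, enlarging the sphere and setting it to overlap all channels.
; Sphere overlaps by the player pawn toggle the hint's visibility.
; Grabbing hides the hint, and dropping shows it again without checking whether the player is still in range.
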(event Custom|BeginOverlap
  (params (OverlappedComponent :type Primitive%20Component%20Object%20Reference) (OtherActor :type Actor%20Object%20Reference) (OtherComp :type Primitive%20Component%20Object%20Reference) (OtherBodyIndex :type Integer) (bFromSweep :type Boolean) (SweepResult :type Hit%20Result%20Structure%20%28by%20ref%29))
  (if (== OtherActor (Game|Player|GetPlayerPawn 0))
    (Rendering|SetVisibility (Variables|Default|GetHintWidgetComponent) true false)))

(event Custom|EndOverlap
  (params (OverlappedComponent :type Primitive%20Component%20Object%20Reference) (OtherActor :type Actor%20Object%20Reference) (OtherComp :type Primitive%20Component%20Object%20Reference) (OtherBodyIndex :type Integer))
  (if (== OtherActor (Game|Player|GetPlayerPawn 0))
    (Rendering|SetVisibility (Variables|Default|GetHintWidgetComponent) false false)))

(event Custom|OnGrabbed
  (Rendering|SetVisibility (Variables|Default|GetHintWidgetComponent) false false))

(event Custom|OnDropped
  (Rendering|SetVisibility (Variables|Default|GetHintWidgetComponent) true false))

(event EventBeginPlay
  (bind _returnvalue (Components|GetOwner))
  (Utilities|FlowControl|Sequence
    (:then_0
      (Variables|Default|SetHintWidgetComponent (Actor|GetComponentbyClass _returnvalue "/Game/Blueprints/Items/BPC_HintWidgetComponent.BPC_HintWidgetComponent_C"))
      (bind _output_get (Variables|Default|SetSphereCollision (Actor|GetComponentbyClass _returnvalue "/Script/Engine.SphereComponent")))
      (Collision|SetCollisionResponsetoAllChannels _output_get "ECR_Overlap")
      (Components|Sphere|SetSphereRadius _output_get 5e+02 true)
      (bind _output_get_2 (Variables|Default|SetgrabComponent (Actor|GetComponentbyClass (Components|GetOwner) "/Game/VRTemplate/Blueprints/GrabComponent.GrabComponent_C")))
      (Utilities|IsValid _output_get_2
        (:Is%20Valid
          (EventDispatchers|BindEventtoOnGrabbed (Variables|Default|GetgrabComponent) (delegate Custom|OnGrabbed))
          (EventDispatchers|BindEventtoOnDropped (Variables|Default|GetgrabComponent) (delegate Custom|OnDropped)))))
    (:then_1
      (Collision|BindEventtoOnComponentBeginOverlap (Variables|Default|GetSphereCollision) (delegate Custom|BeginOverlap))
      (Collision|BindEventtoOnComponentEndOverlap (Variables|Default|GetSphereCollision) (delegate Custom|EndOverlap)))))