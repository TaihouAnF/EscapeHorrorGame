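; BP_Level2Gate is a Level 2 gate that opens when the shadow puzzle is matched.
; On BeginPlay it binds ChangeToGate to the ShadowMatched event of ShadowMatchManager.
; ChangeToGate hides the Cube and plays the OpenGate timeline, whose track Z value is added each update as local yaw to two static meshes in opposite directions, so the rotation accumulates rather than being set absolutely.
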(event Custom|ChangeToGate
  (Rendering|SetVisibility (Variables|Default|GetCube) false false)
  (bind _新建轨道_0 (Timeline|OpenGate PlayFromStart)
    (:Update
      (Transformation|AddLocalRotation (Variables|Default|GetStaticMesh1) (Math|Rotator|MakeRotator 0.0 0.0 (.z _新建轨道_0)) false false)
      (Transformation|AddLocalRotation (Variables|Default|GetStaticMesh) (Math|Rotator|MakeRotator 0.0 0.0 (* (.z _新建轨道_0) -1.0)) false false))))

(event EventBeginPlay
  (EventDispatchers|BindEventtoShadowMatched (Variables|Default|GetShadowMatchManager) (delegate Custom|ChangeToGate)))

(event Collision|EventActorBeginOverlap
  (params (OtherActor :type Actor%20Object%20Reference)))

(event EventTick
  (params (DeltaSeconds :type Float%20%28single-precision%29)))

(fn ConstructionScript)