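; BP_Painting is a puzzle painting that reveals its changed image and opens a bookshelf when the ShadowMatchManager reports a shadow match.
; On the match it swaps the painting material and briefly enables a post process effect.
; It then blends the camera to the BookShelf, slides its Left and Right parts along X with a Timeline, and returns the view to the player pawn.
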(event Custom|ChangePainting
  (bind _bookshelf (Variables|Default|GetBookShelf))
  (bind _camerablendtime (Variables|Default|GetCameraBlendTime))
  (bind _left (Variables|/Game/Blueprints/Painting/BP_Bookshelf.BP_Bookshelf_C|GetLeft _bookshelf))
  (bind _right (Variables|/Game/Blueprints/Painting/BP_Bookshelf.BP_Bookshelf_C|GetRight _bookshelf))
  (bind _relativelocation (Variables|/Script/Engine.SceneComponent|GetRelativeLocation _right))
  (bind _relativelocation_2 (Variables|/Script/Engine.SceneComponent|GetRelativeLocation _left))
  (bind (_x _y _z) (Math|Vector|BreakVector _relativelocation))
  (bind (_x_2 _y_2 _z_2) (Math|Vector|BreakVector _relativelocation_2))
  (Rendering|Material|SetMaterial (Variables|Default|GetPainting) 0 "/Game/Assets/ART_Assets/Material/MI_Painting_Test_After.MI_Painting_Test_After")
  (Variables|/Script/Engine.PostProcessVolume|SetbEnabled (Variables|Default|GetPaintingPostProcess) true)
  (Utilities|FlowControl|Delay 2.0)
  (Variables|/Script/Engine.PostProcessVolume|SetbEnabled (Variables|Default|GetPaintingPostProcess) false)
  (Game|Player|SetViewTargetwithBlend (Game|GetPlayerController 0) (Variables|Default|GetBookShelf) _camerablendtime "VTBlend_Linear" 0.0 false)
  (Utilities|FlowControl|Delay _camerablendtime)
  (bind _newtrack_0 (Timeline|Timeline PlayFromStart)
    (:Update
      (Transformation|SetRelativeLocation _left (Math|Vector|MakeVector (Math|Float|Lerp _x_2 2e+02 _newtrack_0) _y_2 _z_2) false false)
      (Transformation|SetRelativeLocation _right (Math|Vector|MakeVector (Math|Float|Lerp _x -1.5e+02 _newtrack_0) _y _z) false false))
    (:Finished
      (Game|Player|SetViewTargetwithBlend (Game|GetPlayerController 0) (Game|Player|GetPlayerPawn 0) 0.0 "VTBlend_Linear" 0.0 false))))

(event EventBeginPlay
  (EventDispatchers|BindEventtoShadowMatched (Variables|ShadowMatch|GetShadowMatchManager) (delegate Custom|ChangePainting)))

(event Collision|EventActorBeginOverlap
  (params (OtherActor :type Actor%20Object%20Reference)))

(event EventTick
  (params (DeltaSeconds :type Float%20%28single-precision%29)))

(fn ConstructionScript)