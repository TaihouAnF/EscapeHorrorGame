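; Actor component that turns the owner's cast shadow into a collider on a projection plane.
; It projects static mesh vertices along the MovingLight's directional light onto that plane, using a line-traced normal, then offsets vertices with the largest normal-axis extent to add thickness.
; On a timer it recomputes this shape, draws debug spheres, and alternately updates two of the owner's procedural meshes and their convex collision.
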(event EventBeginPlay
  (Variables|Shadow|SetStaticMesh (Actor|GetComponentbyClass (Components|GetOwner) "/Script/Engine.StaticMeshComponent"))
  (CallFunction|GetVertices)
  (CallFunction|GetPlaneNormal)
  (CallFunction|CalculateShadow)
  (CallFunction|ThickenProceduralMesh)
  (CallFunction|CreateMeshComponent))

(event EventTick
  (params (DeltaSeconds :type Float%20%28single-precision%29))
  ;[1 1 1] Check pos
  (if (<= (Variables|Default|GetColliderRefreshTimer) 0.0)
    ;[1 1 1] Timer
    (Variables|Default|SetColliderRefreshTimer (Variables|Shadow|GetColliderRefreshRate))
    (Variables|Default|SetisReversed (not (Variables|Default|GetisReversed)))
    (CallFunction|GetVertices)
    (CallFunction|GetPlaneNormal)
    (CallFunction|CalculateShadow)
    (CallFunction|ThickenProceduralMesh)
    (CallFunction|UpdateProceduralMeshComponent)
    (for _array_element (Variables|Default|GetColliderVertices)
      (Rendering|Debug|DrawDebugSphere _array_element 1e+01 12 "(R=1.000000,G=0.008024,B=0.000000,A=1.000000)" 0.0 1.0))
    (else
      (Variables|Default|SetColliderRefreshTimer (- (Variables|Default|GetColliderRefreshTimer) DeltaSeconds)))))

(fn GetVertices
  (bind _returnvalue (Components|GetOwner))
  (bind _returnvalue_2 (Transformation|GetActorLocation _returnvalue))
  (Utilities|Array|Clear (Variables|Default|GetMeshVertices))
  (bind (_vertices _triangles) (Class|KismetProceduralMeshLibrary|GetSectionfromStaticMesh (Variables|/Script/Engine.StaticMeshComponent|GetStaticMesh (Variables|Shadow|GetStaticMesh))))
  (Variables|Default|SetMeshTriangles _triangles)
  (for _array_element _vertices
    (Utilities|Array|Add (Variables|Default|GetMeshVertices) (+ (Class|KismetMathLibrary|QuatRotateVector (Math|Conversions|ToQuaternion(Rotator) (Transformation|GetActorRotation (Components|GetOwner))) (- (+ _array_element _returnvalue_2) _returnvalue_2)) (Transformation|GetActorLocation (Components|GetOwner))))))

(fn CalculateShadow
  (Utilities|Array|Clear (Variables|Default|GetColliderVertices))
  (for _array_element (Variables|Default|GetMeshVertices)
    (bind _output_get (Variables|Temp|Settempvec _array_element))
    (bind _t (CallFunction|GetProjectionT))
    (Variables|Temp|Settempt _t)
    (Utilities|Array|Add (Variables|Default|GetColliderVertices) (Math|Vector|MakeVector (- (.X (Math|Vector|BreakVector _output_get)) (* (Variables|Temp|Gettempt) (.X (Math|Vector|BreakVector (Math|Vector|GetForwardVector (Actor|GetComponentbyClass (Variables|Shadow|GetMovingLight) "/Script/Engine.DirectionalLightComponent")))))) (- (.Y (Math|Vector|BreakVector _output_get)) (* (Variables|Temp|Gettempt) (.Y (Math|Vector|BreakVector (Math|Vector|GetForwardVector (Actor|GetComponentbyClass (Variables|Shadow|GetMovingLight) "/Script/Engine.DirectionalLightComponent")))))) (- (.Z (Math|Vector|BreakVector _output_get)) (* (Variables|Temp|Gettempt) (.Z (Math|Vector|BreakVector (Math|Vector|GetForwardVector (Actor|GetComponentbyClass (Variables|Shadow|GetMovingLight) "/Script/Engine.DirectionalLightComponent"))))))))))

(fn GetPlaneNormal
  (bind _outhit (Collision|LineTraceByChannel (Transformation|GetActorLocation (Components|GetOwner)) (Transformation|GetActorLocation (Variables|Shadow|GetProjectionPlane)) "TraceTypeQuery3" false 0 "None"))
  (Variables|Default|SetPlaneNormal (.Normal (Collision|BreakHitResult _outhit))))

(fn GetProjectionT
  (return (/ (- (+ (+ (* (.X (Math|Vector|BreakVector (Variables|Temp|Gettempvec))) (.X (Math|Vector|BreakVector (Variables|Default|GetPlaneNormal)))) (* (.Y (Math|Vector|BreakVector (Variables|Temp|Gettempvec))) (.Y (Math|Vector|BreakVector (Variables|Default|GetPlaneNormal))))) (* (.Z (Math|Vector|BreakVector (Variables|Temp|Gettempvec))) (.Z (Math|Vector|BreakVector (Variables|Default|GetPlaneNormal))))) (+ (+ (+ (* (.X (Math|Vector|BreakVector (Transformation|GetActorLocation (Variables|Shadow|GetProjectionPlane)))) (.X (Math|Vector|BreakVector (Variables|Default|GetPlaneNormal)))) (* (.Y (Math|Vector|BreakVector (Transformation|GetActorLocation (Variables|Shadow|GetProjectionPlane)))) (.Y (Math|Vector|BreakVector (Variables|Default|GetPlaneNormal))))) (* (.Z (Math|Vector|BreakVector (Transformation|GetActorLocation (Variables|Shadow|GetProjectionPlane)))) (.Z (Math|Vector|BreakVector (Variables|Default|GetPlaneNormal))))) (Variables|Shadow|GetSurfaceOffset))) (+ (+ (* (.X (Math|Vector|BreakVector (Variables|Default|GetPlaneNormal))) (.X (Math|Vector|BreakVector (Math|Vector|GetForwardVector (Actor|GetComponentbyClass (Variables|Shadow|GetMovingLight) "/Script/Engine.DirectionalLightComponent"))))) (* (.Y (Math|Vector|BreakVector (Variables|Default|GetPlaneNormal))) (.Y (Math|Vector|BreakVector (Math|Vector|GetForwardVector (Actor|GetComponentbyClass (Variables|Shadow|GetMovingLight) "/Script/Engine.DirectionalLightComponent")))))) (* (.Z (Math|Vector|BreakVector (Variables|Default|GetPlaneNormal))) (.Z (Math|Vector|BreakVector (Math|Vector|GetForwardVector (Actor|GetComponentbyClass (Variables|Shadow|GetMovingLight) "/Script/Engine.DirectionalLightComponent")))))))))

(fn CreateMeshComponent
  (bind _output_get (Variables|Shadow|SetProceduralMeshes (Actor|GetComponentsByClass (Components|GetOwner) "/Script/ProceduralMeshComponent.ProceduralMeshComponent")))
  (for _array_element _output_get
    (Class|ProceduralMeshComponent|CreateMeshSectionLinearColor _array_element 0 (Variables|Default|GetColliderVertices) (Variables|Default|GetMeshTriangles) 0 0 0 0 0 0 0 true false)
    (Variables|/Script/Engine.SceneComponent|SetbAbsoluteRotation _array_element true)
    (Rendering|Components|SetLightingChannels _array_element false true false)))

(fn UpdateProceduralMeshComponent
  (bind _returnvalue (Components|GetOwner))
  (bind _collidervertices (Variables|Default|GetColliderVertices))
  (bind _returnvalue_2 (Actor|GetComponentsByClass _returnvalue "/Script/ProceduralMeshComponent.ProceduralMeshComponent"))
  (bind _output (Utilities|Array|Get(acopy) _returnvalue_2 1))
  (bind _output_2 (Utilities|Array|Get(acopy) _returnvalue_2))
  (for (_array_element _array_index) _collidervertices
    (Utilities|Array|SetArrayElem _collidervertices _array_index (- _array_element (Transformation|GetActorLocation (Components|GetOwner)))))
  (if (Variables|Default|GetisReversed)
    (Class|ProceduralMeshComponent|UpdateMeshSectionLinearColor _output_2 0 (Variables|Default|GetColliderVertices) 0 0 0 0 0 0 0 true)
    (Class|ProceduralMeshComponent|ClearCollisionConvexMeshes _output_2)
    (Class|ProceduralMeshComponent|AddCollisionConvexMesh _output_2 (Variables|Default|GetColliderVertices))
    (else
      (Class|ProceduralMeshComponent|UpdateMeshSectionLinearColor _output 0 (Variables|Default|GetColliderVertices) 0 0 0 0 0 0 0 true)
      (Class|ProceduralMeshComponent|ClearCollisionConvexMeshes _output)
      (Class|ProceduralMeshComponent|AddCollisionConvexMesh _output (Variables|Default|GetColliderVertices)))))

(fn ThickenProceduralMesh
  (bind _planenormal (Variables|Default|GetPlaneNormal))
  (bind _planenormal_2 (Variables|Default|GetPlaneNormal))
  (bind _collidervertices (Variables|Default|GetColliderVertices))
  (Utilities|Array|Clear (Variables|Temp|GettempIndecies))
  (Variables|Temp|SettempMax 0.0)
  (for _array_element (Variables|Default|GetMeshVertices)
    (if (> (Math|Vector|VectorLength (* (/ (Math|Vector|DotProduct _array_element _planenormal) (Math|Float|Square (Math|Vector|VectorLength _planenormal))) (Variables|Default|GetPlaneNormal))) (Variables|Temp|GettempMax))
      (Variables|Temp|SettempMax (Math|Vector|VectorLength (* (/ (Math|Vector|DotProduct _array_element _planenormal) (Math|Float|Square (Math|Vector|VectorLength _planenormal))) (Variables|Default|GetPlaneNormal))))))
  (for (_array_element_2 _array_index) (Variables|Default|GetMeshVertices)
    (if (< (Math|Float|Absolute(Float) (- (Variables|Temp|GettempMax) (Math|Vector|VectorLength (* (/ (Math|Vector|DotProduct _array_element_2 _planenormal_2) (Math|Float|Square (Math|Vector|VectorLength _planenormal_2))) (Variables|Default|GetPlaneNormal))))) 0.01)
      (Utilities|Array|Add (Variables|Temp|GettempIndecies) _array_index)))
  ;[1 1 1] Change the thickness of procedural mesh, if want to adjust the shape of mesh, change here
  (for _array_element_3 (Variables|Temp|GettempIndecies)
    (Utilities|Array|SetArrayElem _collidervertices _array_element_3 (+ (Utilities|Array|Get(acopy) _collidervertices _array_element_3) (* (Variables|Default|GetPlaneNormal) (Variables|Shadow|GetShadowColliderThickness))))))