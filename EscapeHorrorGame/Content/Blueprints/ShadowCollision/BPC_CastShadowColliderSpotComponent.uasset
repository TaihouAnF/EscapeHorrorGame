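; Actor component that turns the shadow its owner's static mesh casts from a spot light into solid procedural mesh collision.
; It traces toward the ProjectionPlane actor for a surface normal and point, then projects rotated mesh vertices along light rays onto that plane.
; Vertices farthest along the normal are offset for thickness.
; Owner movement, but not light movement, triggers recalculation, updating the procedural mesh and its convex collision.
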(event EventBeginPlay
  (Variables|Shadow|SetSpotLight (Actor|GetComponentbyClass (Variables|Shadow|GetSpotLightActor) "/Script/Engine.SpotLightComponent"))
  (Variables|Shadow|SetStaticMesh (Actor|GetComponentbyClass (Components|GetOwner) "/Script/Engine.StaticMeshComponent"))
  (CallFunction|GetVertices)
  (CallFunction|GetPlaneNormal)
  (CallFunction|CalculateShadow)
  (CallFunction|ThickenProceduralMesh)
  (CallFunction|CreateMeshComponent))

(event EventTick
  (params (DeltaSeconds :type Float%20%28single-precision%29))
  ;[1 1 1] Check pos
  (if (> (Math|Float|Absolute(Float) (Math|Vector|Distance(Vector) (Transformation|GetActorLocation (Components|GetOwner)) (Variables|Default|GetLastPos))) 1.0)
    (Variables|Default|SetLastPos (Transformation|GetActorLocation (Components|GetOwner)))
    (CallFunction|GetVertices)
    (CallFunction|GetPlaneNormal)
    (CallFunction|CalculateShadow)
    (CallFunction|ThickenProceduralMesh)
    (CallFunction|UpdateProceduralMeshComponent)))

(fn GetVertices
  (bind _returnvalue (Components|GetOwner))
  (bind _returnvalue_2 (Transformation|GetActorLocation _returnvalue))
  (Utilities|Array|Clear (Variables|Default|GetMeshVertices))
  (bind (_vertices _triangles) (Class|KismetProceduralMeshLibrary|GetSectionfromStaticMesh (Variables|/Script/Engine.StaticMeshComponent|GetStaticMesh (Variables|Shadow|GetStaticMesh))))
  (Variables|Default|SetMeshTriangles _triangles)
  (for _array_element _vertices
    (Utilities|Array|Add (Variables|Default|GetMeshVertices) (+ (Class|KismetMathLibrary|QuatRotateVector (Math|Conversions|ToQuaternion(Rotator) (Transformation|GetActorRotation (Components|GetOwner))) (- (+ _array_element _returnvalue_2) _returnvalue_2)) (Transformation|GetActorLocation (Components|GetOwner))))))

(fn CalculateShadow
  (Utilities|Array|Clear (Variables|Default|GetColliderVertices))
  (for _array_element (Variables|Default|GetMeshVertices)
    (bind _output_get (Variables|Temp|Settempvec _array_element))
    (bind _t (CallFunction|GetProjectionT _output_get))
    (Variables|Temp|Settempt _t)
    (Utilities|Array|Add (Variables|Default|GetColliderVertices) (Math|Vector|MakeVector (- (.X (Math|Vector|BreakVector _output_get)) (* (Variables|Temp|Gettempt) (.X (Math|Vector|BreakVector (- (Variables|Temp|Gettempvec) (Transformation|GetWorldLocation (Variables|Shadow|GetSpotLight))))))) (- (.Y (Math|Vector|BreakVector _output_get)) (* (Variables|Temp|Gettempt) (.Y (Math|Vector|BreakVector (- (Variables|Temp|Gettempvec) (Transformation|GetWorldLocation (Variables|Shadow|GetSpotLight))))))) (- (.Z (Math|Vector|BreakVector _output_get)) (* (Variables|Temp|Gettempt) (.Z (Math|Vector|BreakVector (- (Variables|Temp|Gettempvec) (Transformation|GetWorldLocation (Variables|Shadow|GetSpotLight)))))))))))

(fn GetPlaneNormal
  (bind (_outhit _returnvalue) (Collision|LineTraceByChannel (Transformation|GetActorLocation (Components|GetOwner)) (Transformation|GetActorLocation (Variables|Shadow|GetProjectionPlane)) "TraceTypeQuery3" false 0 "None"))
  (if _returnvalue
    (Variables|Shadow|SetPlaneNormal (.Normal (Collision|BreakHitResult _outhit)))
    (Variables|Shadow|SetPlaneLocation (.Location (Collision|BreakHitResult _outhit)))
    (else
      (for _array_element (Actor|GetComponentsByClass (Variables|Shadow|GetProjectionPlane) "/Script/Engine.StaticMeshComponent")
        (bind (_outhit_2 _returnvalue_2) (Collision|LineTraceByChannel (Transformation|GetActorLocation (Components|GetOwner)) (Transformation|GetWorldLocation _array_element) "TraceTypeQuery3" false 0 "None"))
        (if _returnvalue_2
          (Variables|Shadow|SetPlaneNormal (.Normal (Collision|BreakHitResult _outhit_2)))
          (Variables|Shadow|SetPlaneLocation (.Location (Collision|BreakHitResult _outhit_2)))
          (return))))))

(fn GetProjectionT
  (params (vetex :type Vector))
  (bind (_x _y _z) (Math|Vector|BreakVector vetex))
  (return (/ (- (+ (+ (* (.X (Math|Vector|BreakVector (Variables|Temp|Gettempvec))) (.X (Math|Vector|BreakVector (Variables|Shadow|GetPlaneNormal)))) (* (.Y (Math|Vector|BreakVector (Variables|Temp|Gettempvec))) (.Y (Math|Vector|BreakVector (Variables|Shadow|GetPlaneNormal))))) (* (.Z (Math|Vector|BreakVector (Variables|Temp|Gettempvec))) (.Z (Math|Vector|BreakVector (Variables|Shadow|GetPlaneNormal))))) (+ (+ (+ (* (.X (Math|Vector|BreakVector (Variables|Shadow|GetPlaneLocation))) (.X (Math|Vector|BreakVector (Variables|Shadow|GetPlaneNormal)))) (* (.Y (Math|Vector|BreakVector (Variables|Shadow|GetPlaneLocation))) (.Y (Math|Vector|BreakVector (Variables|Shadow|GetPlaneNormal))))) (* (.Z (Math|Vector|BreakVector (Variables|Shadow|GetPlaneLocation))) (.Z (Math|Vector|BreakVector (Variables|Shadow|GetPlaneNormal))))) (Variables|Shadow|GetSurfaceOffset))) (+ (+ (* (.X (Math|Vector|BreakVector (Variables|Shadow|GetPlaneNormal))) (- _x (.X (Math|Vector|BreakVector (Transformation|GetWorldLocation (Variables|Shadow|GetSpotLight)))))) (* (.Y (Math|Vector|BreakVector (Variables|Shadow|GetPlaneNormal))) (- _y (.Y (Math|Vector|BreakVector (Transformation|GetWorldLocation (Variables|Shadow|GetSpotLight))))))) (* (.Z (Math|Vector|BreakVector (Variables|Shadow|GetPlaneNormal))) (- _z (.Z (Math|Vector|BreakVector (Transformation|GetWorldLocation (Variables|Shadow|GetSpotLight))))))))))

(fn CreateMeshComponent
  (for _array_element (Variables|Shadow|GetProceduralMeshIndex)
    (Utilities|Array|Add (Variables|Shadow|GetProceduralMeshes) (Utilities|Array|Get(acopy) (Actor|GetComponentsByClass (Components|GetOwner) "/Script/ProceduralMeshComponent.ProceduralMeshComponent") _array_element)))
  (for _array_element_2 (Variables|Shadow|GetProceduralMeshes)
    (Class|ProceduralMeshComponent|CreateMeshSectionLinearColor _array_element_2 0 (Variables|Default|GetColliderVertices) (Variables|Default|GetMeshTriangles) 0 0 0 0 0 0 0 true false)
    (Variables|/Script/Engine.SceneComponent|SetbAbsoluteRotation _array_element_2 true)))

(fn UpdateProceduralMeshComponent
  (bind _returnvalue (Components|GetOwner))
  (bind _proceduralmeshindex (Variables|Shadow|GetProceduralMeshIndex))
  (bind _collidervertices (Variables|Default|GetColliderVertices))
  (bind _proceduralmeshindex_2 (Variables|Shadow|GetProceduralMeshIndex))
  (bind _returnvalue_2 (Actor|GetComponentsByClass _returnvalue "/Script/ProceduralMeshComponent.ProceduralMeshComponent"))
  (bind _output (Utilities|Array|Get(acopy) _proceduralmeshindex 1))
  (bind _output_2 (Utilities|Array|Get(acopy) _proceduralmeshindex_2))
  (bind _output_3 (Utilities|Array|Get(acopy) _returnvalue_2 _output))
  (bind _output_4 (Utilities|Array|Get(acopy) _returnvalue_2 _output_2))
  (for (_array_element _array_index) _collidervertices
    (Utilities|Array|SetArrayElem _collidervertices _array_index (- _array_element (Transformation|GetActorLocation (Components|GetOwner)))))
  (if (Variables|Default|GetisReversed)
    (Class|ProceduralMeshComponent|UpdateMeshSectionLinearColor _output_4 0 (Variables|Default|GetColliderVertices) 0 0 0 0 0 0 0 true :!label _label)
    (Class|ProceduralMeshComponent|ClearCollisionConvexMeshes _output_4)
    (Class|ProceduralMeshComponent|AddCollisionConvexMesh _output_4 (Variables|Default|GetColliderVertices))
    (elif (> (Utilities|Array|Length (Variables|Shadow|GetProceduralMeshIndex)) 1)
      (Class|ProceduralMeshComponent|UpdateMeshSectionLinearColor _output_3 0 (Variables|Default|GetColliderVertices) 0 0 0 0 0 0 0 true)
      (Class|ProceduralMeshComponent|ClearCollisionConvexMeshes _output_3)
      (Class|ProceduralMeshComponent|AddCollisionConvexMesh _output_3 (Variables|Default|GetColliderVertices))
      (else
        (goto _label)))))

(fn ThickenProceduralMesh
  (bind _planenormal (Variables|Shadow|GetPlaneNormal))
  (bind _planenormal_2 (Variables|Shadow|GetPlaneNormal))
  (bind _collidervertices (Variables|Default|GetColliderVertices))
  (Utilities|Array|Clear (Variables|Temp|GettempIndeciesMax))
  (Variables|Temp|SettempMax 0.0)
  (for _array_element (Variables|Default|GetMeshVertices)
    (if (> (Math|Vector|VectorLength (* (/ (Math|Vector|DotProduct _array_element _planenormal) (Math|Float|Square (Math|Vector|VectorLength _planenormal))) (Variables|Shadow|GetPlaneNormal))) (Variables|Temp|GettempMax))
      (Variables|Temp|SettempMax (Math|Vector|VectorLength (* (/ (Math|Vector|DotProduct _array_element _planenormal) (Math|Float|Square (Math|Vector|VectorLength _planenormal))) (Variables|Shadow|GetPlaneNormal))))))
  (for (_array_element_2 _array_index) (Variables|Default|GetMeshVertices)
    (if (< (Math|Float|Absolute(Float) (- (Variables|Temp|GettempMax) (Math|Vector|VectorLength (* (/ (Math|Vector|DotProduct _array_element_2 _planenormal_2) (Math|Float|Square (Math|Vector|VectorLength _planenormal_2))) (Variables|Shadow|GetPlaneNormal))))) 0.01)
      (Utilities|Array|Add (Variables|Temp|GettempIndeciesMax) _array_index)))
  ;[1 1 1] Change the thickness of procedural mesh, if want to adjust the shape of mesh, change here
  (for _array_element_3 (Variables|Temp|GettempIndeciesMax)
    (Utilities|Array|SetArrayElem _collidervertices _array_element_3 (+ (Utilities|Array|Get(acopy) _collidervertices _array_element_3) (* (Variables|Shadow|GetPlaneNormal) (Variables|Shadow|GetShadowColliderThickness))))))