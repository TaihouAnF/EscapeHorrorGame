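; Base grabbable spot actor for the shadow-collision system, with a hint widget and a sphere component.
; On BeginPlay it enables player input and sets both components to the hint widget world scale.
; W and S set a vertical MoveDir, cleared on release, though nothing in this file applies it.
; Tick offsets the actor and immediately reverses it without sweep, a net-zero nudge that presumably forces a transform update.
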(event EventBeginPlay
  (Input|EnableInput (Game|GetPlayerController 0))
  (Transformation|SetWorldScale3D (Variables|Default|GetBPC_HintWidgetComponent) (Variables|Default|GetHintWidgetScale))
  (Transformation|SetWorldScale3D (Variables|Default|GetSphere) (Variables|Default|GetHintWidgetScale)))

(event Collision|EventActorBeginOverlap
  (params (OtherActor :type Actor%20Object%20Reference)))

(event EventTick
  (params (DeltaSeconds :type Float%20%28single-precision%29))
  (Transformation|AddActorWorldOffset "1.000000,1.000000,0.000000")
  (Transformation|AddActorWorldOffset "-1.000000,-1.000000,0.000000"))

(event Input|KeyboardEvents|S
  (params (Key :type Key%20Structure :default "None"))
  (:Pressed
    (Variables|Default|SetMoveDir "0.000000,0.000000,-1.000000"))
  (:Released
    (Variables|Default|SetMoveDir "0, 0, 0")))

(event Input|KeyboardEvents|W
  (params (Key :type Key%20Structure :default "None"))
  (:Pressed
    (Variables|Default|SetMoveDir "0.000000,0.000000,1.000000"))
  (:Released
    (Variables|Default|SetMoveDir "0, 0, 0")))

(fn ConstructionScript)