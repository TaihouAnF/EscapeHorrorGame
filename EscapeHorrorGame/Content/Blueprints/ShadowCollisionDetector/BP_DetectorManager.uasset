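; Shadow-shape puzzle manager that detects when a shadow fits the outline defined by an inner and an outer spline.
; On BeginPlay it spawns detector points at each spline point and registers itself as their parent.
; InnerDetected and OuterDetected recount occupied points.
; Tick requires all inner and no outer points occupied for a brief hold, then latches completion and fires ShadowMatched.
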(event EventBeginPlay
  (bind _outerspline (Variables|Default|GetOuterSpline))
  (bind _innerspline (Variables|Default|GetInnerSpline))
  (Utilities|FlowControl|Sequence
    (:then_0
      (for _index (range 0 (- (Spline|GetNumberOfSplinePoints _innerspline) 1))
        (bind _returnvalue (Game|SpawnActorfromClass "/Game/Blueprints/ShadowCollisionDetector/BP_InnerDetectorPoint.BP_InnerDetectorPoint_C" (Spline|GetTransformatSplinePoint _innerspline _index "World" false) "Undefined" "MultiplyWithRoot" 0 0))
        (Utilities|Array|Add (Variables|Default|GetInnerDetectorPoints) _returnvalue)
        (Default|RegisterParent _returnvalue self)
        (Variables|Default|SetMaxInnerDetectorPointNumber (+ (Variables|Default|GetMaxInnerDetectorPointNumber) 1))))
    (:then_1
      (for _index_2 (range 0 (- (Spline|GetNumberOfSplinePoints _outerspline) 1))
        (bind _returnvalue_2 (Game|SpawnActorfromClass "/Game/Blueprints/ShadowCollisionDetector/BP_OuterDetectorPoint.BP_OuterDetectorPoint_C" (Spline|GetTransformatSplinePoint _outerspline _index_2 "World" false) "Undefined" "MultiplyWithRoot" 0 0))
        (Utilities|Array|Add (Variables|Default|GetOuterDetectorPoints) _returnvalue_2)
        (Default|RegisterParent _returnvalue_2 self)
        (Variables|Default|SetMaxOuterDetectorPointNumber (+ (Variables|Default|GetMaxOuterDetectorPointNumber) 1))))))

(event Collision|EventActorBeginOverlap
  (params (OtherActor :type Actor%20Object%20Reference)))

(event EventTick
  (params (DeltaSeconds :type Float%20%28single-precision%29))
  (if (not (Variables|Default|GetCompleteMatch))
    (CallFunction|EvaluateShadowDetectResult)
    (if (Variables|Default|GetIsMatched)
      (Variables|Default|SetMatchTime (+ (Variables|Default|GetMatchTime) DeltaSeconds))
      (if (> (Variables|Default|GetMatchTime) 0.1)
        (Variables|Default|SetCompleteMatch true)
        (Default|CallShadowMatched)
        (Development|PrintString "Shadow Shape correct!"))
      (else
        (Variables|Default|SetMatchTime 0.0)))))

(fn ConstructionScript)

(fn InnerDetected
  (if (not (Variables|Default|GetCompleteMatch))
    (Variables|Default|SetCurInnerDetectorPointNumber 0)
    (for _array_element (Variables|Default|GetInnerDetectorPoints)
      (if (Variables|/Game/Blueprints/ShadowCollisionDetector/BP_InnerDetectorPoint.BP_InnerDetectorPoint_C|GetIsOccupied _array_element)
        (Variables|Default|SetCurInnerDetectorPointNumber (+ (Variables|Default|GetCurInnerDetectorPointNumber) 1))))))

(fn OuterDetected
  (if (not (Variables|Default|GetCompleteMatch))
    (Variables|Default|SetCurOuterDetectorPointNumber 0)
    (for _array_element (Variables|Default|GetOuterDetectorPoints)
      (if (Variables|/Game/Blueprints/ShadowCollisionDetector/BP_OuterDetectorPoint.BP_OuterDetectorPoint_C|GetIsOccupied _array_element)
        (Variables|Default|SetCurOuterDetectorPointNumber (+ (Variables|Default|GetCurOuterDetectorPointNumber) 1))))))

(fn EvaluateShadowDetectResult
  (if (> (Variables|Default|GetCurOuterDetectorPointNumber) 0)
    (Variables|Default|SetIsMatched false)
    (Variables|Default|SetMatchTime 0.0)
    (elif (== (Variables|Default|GetMaxInnerDetectorPointNumber) (Variables|Default|GetCurInnerDetectorPointNumber))
      (Variables|Default|SetIsMatched true)
      (else
        (Variables|Default|SetIsMatched false)
        (Variables|Default|SetMatchTime 0.0)))))