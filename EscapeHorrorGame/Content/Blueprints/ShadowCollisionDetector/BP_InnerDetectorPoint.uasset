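; BP_InnerDetectorPoint is an inner sensor point for shadow collision detection that tracks whether a procedural mesh overlaps its sphere.
; On begin and end overlap it sets IsOccupied and applies a dynamic grid material to its static mesh, red when occupied and gray when clear.
; Either change calls InnerDetected on the DetectorManager supplied through RegisterParent, if that reference is valid.
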(event OnComponentBeginOverlap(Sphere)
  (params (OverlappedComponent :type Primitive%20Component%20Object%20Reference) (OtherActor :type Actor%20Object%20Reference) (OtherComp :type Primitive%20Component%20Object%20Reference) (OtherBodyIndex :type Integer) (bFromSweep :type Boolean) (SweepResult :type Hit%20Result%20Structure%20%28by%20ref%29))
  (bind _detectormanager (Variables|Default|GetDetectorManager))
  (Utilities|Casting|CastToProceduralMeshComponent OtherComp)
  (bind _returnvalue (Rendering|Material|CreateDynamicMaterialInstance (Variables|Default|GetStaticMesh) 0 "/Game/Assets/SuperGrid/StarterPack/Materials/Palette/Grids/M_SuperGrid_White.M_SuperGrid_White" "None" :!class /Script/Engine.PrimitiveComponent))
  (Rendering|Material|SetVectorParameterValue _returnvalue "Color" (Math|Color|MakeColor 1.0 0.0 0.0) :!class /Script/Engine.MaterialInstanceDynamic)
  (Variables|Default|SetIsOccupied true)
  (Utilities|IsValid _detectormanager
    (:Is%20Valid
      (Default|InnerDetected _detectormanager))))

(event OnComponentEndOverlap(Sphere)
  (params (OverlappedComponent :type Primitive%20Component%20Object%20Reference) (OtherActor :type Actor%20Object%20Reference) (OtherComp :type Primitive%20Component%20Object%20Reference) (OtherBodyIndex :type Integer))
  (bind _detectormanager (Variables|Default|GetDetectorManager))
  (Utilities|Casting|CastToProceduralMeshComponent OtherComp)
  (bind _returnvalue (Rendering|Material|CreateDynamicMaterialInstance (Variables|Default|GetStaticMesh) 0 "/Game/Assets/SuperGrid/StarterPack/Materials/Palette/Grids/M_SuperGrid_White.M_SuperGrid_White" "None" :!class /Script/Engine.PrimitiveComponent))
  (Rendering|Material|SetVectorParameterValue _returnvalue "Color" (Math|Color|MakeColor 0.28 0.28 0.28) :!class /Script/Engine.MaterialInstanceDynamic)
  (Variables|Default|SetIsOccupied false)
  (Utilities|IsValid _detectormanager
    (:Is%20Valid
      (Default|InnerDetected _detectormanager))))

(event EventBeginPlay)

(event Collision|EventActorBeginOverlap
  (params (OtherActor :type Actor%20Object%20Reference)))

(event EventTick
  (params (DeltaSeconds :type Float%20%28single-precision%29)))

(fn ConstructionScript)

(fn RegisterParent
  (params (DetectorManager :type BP%20Detector%20Manager%20Object%20Reference))
  (Variables|Default|SetDetectorManager DetectorManager))